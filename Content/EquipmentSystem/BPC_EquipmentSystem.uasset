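; Player equipment component for BP_ThirdPersonCharacter that handles item pickup and the equipment and general inventory panels.
; Interact sphere-traces from the follow camera, stores weapon or consumable data in slot arrays, notifies the general inventory widget of consumables, and destroys the pickup.
; Two inputs toggle lazily created widgets through one shared open flag, switching cursor and input mode and disabling movement and attacks while open.
; GetConsumable is an empty stub.
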(event Input|EnhancedActionEvents|EnhancedInputActionIA_Interact
  (params (ActionValue :type Boolean) (ElapsedSeconds :type Float%20%28double-precision%29) (TriggeredSeconds :type Float%20%28double-precision%29) (InputAction :type Input%20Action%20Object%20Reference :default "/Game/ThirdPerson/Input/Actions/IA_Interact.IA_Interact"))
  (bind _follow_camera (Variables|Default|GetFollow%20Camera))
  (bind _as_bp_third_person_character (Variables|Default|GetAs%20BP%20Third%20Person%20Character))
  (bind _returnvalue (Transformation|GetWorldLocation _follow_camera))
  (bind _bpc_equipmentsystem (Variables|/Game/ThirdPerson/Blueprints/BP_ThirdPersonCharacter.BP_ThirdPersonCharacter_C|GetBPC_EquipmentSystem _as_bp_third_person_character))
  ;[1 1 1] Pick Up Trace
  (:Started
    (bind (_outhit _returnvalue_2) (Collision|SphereTraceForObjects _returnvalue (+ _returnvalue (* (Math|Vector|GetForwardVector (Transformation|GetWorldRotation _follow_camera)) 1e+03)) 6e+01 (Utilities|Array|MakeArray "ObjectTypeQuery2") false 0 "ForDuration"))
    (if _returnvalue_2
      (Utilities|FlowControl|Sequence
        (:then_0
          (bind _asbp_weapon (Utilities|Casting|CastToBP_Weapon (.HitActor (Collision|BreakHitResult _outhit)))
            (:then
              (CallFunction|AddWeapon (Variables|/Game/EquipmentSystem/BP_Weapon.BP_Weapon_C|GetItem%20Data _asbp_weapon))
              (Actor|DestroyActor _asbp_weapon))
            (:CastFailed
              (bind _asbp_consumables (Utilities|Casting|CastToBP_Consumables (.HitActor (Collision|BreakHitResult _outhit))))
              (CallFunction|AddConsumable (Variables|/Game/EquipmentSystem/BP_Consumables.BP_Consumables_C|GetItemData%28Consumables%29 _asbp_consumables))
              (Development|PrintString (Utilities|GetDisplayName (Variables|BPC_EquipmentSystem_C|GetGeneralInventory _bpc_equipmentsystem)))
              (Default|ConsumableAdded (Variables|BPC_EquipmentSystem_C|GetGeneralInventory _bpc_equipmentsystem) (Variables|/Game/EquipmentSystem/BP_Consumables.BP_Consumables_C|GetItemData%28Consumables%29 _asbp_consumables))
              (Actor|DestroyActor _asbp_consumables)))
          (Development|PrintString "Item Gathered"))))))

(event Input|EnhancedActionEvents|EnhancedInputActionIA_OpenInventory
  (params (ActionValue :type Boolean) (ElapsedSeconds :type Float%20%28double-precision%29) (TriggeredSeconds :type Float%20%28double-precision%29) (InputAction :type Input%20Action%20Object%20Reference :default "/Game/ThirdPerson/Input/Actions/IA_OpenInventory.IA_OpenInventory"))
  (bind _returnvalue (Game|GetPlayerController 0))
  ;[1 1 1] Equipment Menu Panel
  (:Started
    (if (not (Variables|Default|GetIsPanelOpen?))
      (Variables|Default|SetIsPanelOpen? true)
      (bind _equipmentwidget (Variables|Default|GetEquipmentWidget)
        (:then
          (Widget|SetVisibility _equipmentwidget "Visible"))
        (:else
          (bind _returnvalue_2 (UserInterface|CreateWidget "/Game/EquipmentSystem/Ui/WB_Equipment.WB_Equipment_C"))
          (bind _output_get (Variables|Default|SetEquipmentWidget _returnvalue_2))
          (UserInterface|Viewport|AddtoViewport _output_get 0)))
      (Variables|/Script/Engine.PlayerController|SetbShowMouseCursor _returnvalue true)
      (Input|SetInputModeGameandUI _returnvalue (Variables|Default|GetEquipmentWidget) "DoNotLock" true false)
      (bind _asbp_third_person_character (Utilities|Casting|CastToBP_ThirdPersonCharacter (Components|GetOwner)))
      (Pawn|Components|CharacterMovement|SetMovementMode (Variables|/Script/Engine.Character|GetCharacterMovement _asbp_third_person_character) "MOVE_None" 0)
      (bind _asbp_third_person_character_2 (Utilities|Casting|CastToBP_ThirdPersonCharacter (Components|GetOwner)))
      (Variables|/Game/Blueprints/BPC_AttackSystem.BPC_AttackSystem_C|SetCanAttack? (Variables|/Game/ThirdPerson/Blueprints/BP_ThirdPersonCharacter.BP_ThirdPersonCharacter_C|GetBPC_AttackSystem _asbp_third_person_character_2) false)
      (else
        (Variables|Default|SetIsPanelOpen? false)
        (bind _equipmentwidget_2 (Variables|Default|GetEquipmentWidget)
          (:then
            (Widget|SetVisibility _equipmentwidget_2 "Hidden")
            (Variables|/Script/Engine.PlayerController|SetbShowMouseCursor _returnvalue false)
            (Input|SetInputModeGameOnly _returnvalue false)
            (bind _asbp_third_person_character_3 (Utilities|Casting|CastToBP_ThirdPersonCharacter (Components|GetOwner)))
            (Pawn|Components|CharacterMovement|SetMovementMode (Variables|/Script/Engine.Character|GetCharacterMovement _asbp_third_person_character_3) "MOVE_Walking" 0)
            (bind _asbp_third_person_character_4 (Utilities|Casting|CastToBP_ThirdPersonCharacter (Components|GetOwner)))
            (Variables|/Game/Blueprints/BPC_AttackSystem.BPC_AttackSystem_C|SetCanAttack? (Variables|/Game/ThirdPerson/Blueprints/BP_ThirdPersonCharacter.BP_ThirdPersonCharacter_C|GetBPC_AttackSystem _asbp_third_person_character_4) true))
          (:else))))))

(event Input|EnhancedActionEvents|EnhancedInputActionIA_GeneralInventory
  (params (ActionValue :type Boolean) (ElapsedSeconds :type Float%20%28double-precision%29) (TriggeredSeconds :type Float%20%28double-precision%29) (InputAction :type Input%20Action%20Object%20Reference :default "/Game/ThirdPerson/Input/Actions/IA_GeneralInventory.IA_GeneralInventory"))
  (bind _returnvalue (Game|GetPlayerController 0))
  (:Started
    (if (not (Variables|Default|GetIsPanelOpen?))
      (Variables|Default|SetIsPanelOpen? true)
      (bind _generalinventory (Variables|Default|GetGeneralInventory)
        (:then
          (Widget|SetVisibility _generalinventory "Visible"))
        (:else
          (bind _returnvalue_2 (UserInterface|CreateWidget "/Game/EquipmentSystem/Ui/WB_GeneralEquipment.WB_GeneralEquipment_C"))
          (bind _output_get (Variables|Default|SetGeneralInventory _returnvalue_2))
          (UserInterface|Viewport|AddtoViewport _output_get 0)))
      (Variables|/Script/Engine.PlayerController|SetbShowMouseCursor _returnvalue true)
      (Input|SetInputModeGameandUI _returnvalue (Variables|Default|GetGeneralInventory) "DoNotLock" true false)
      (bind _asbp_third_person_character (Utilities|Casting|CastToBP_ThirdPersonCharacter (Components|GetOwner)))
      (Pawn|Components|CharacterMovement|SetMovementMode (Variables|/Script/Engine.Character|GetCharacterMovement _asbp_third_person_character) "MOVE_None" 0)
      (bind _asbp_third_person_character_2 (Utilities|Casting|CastToBP_ThirdPersonCharacter (Components|GetOwner)))
      (Variables|/Game/Blueprints/BPC_AttackSystem.BPC_AttackSystem_C|SetCanAttack? (Variables|/Game/ThirdPerson/Blueprints/BP_ThirdPersonCharacter.BP_ThirdPersonCharacter_C|GetBPC_AttackSystem _asbp_third_person_character_2) false)
      (else
        (Variables|Default|SetIsPanelOpen? false)
        (bind _generalinventory_2 (Variables|Default|GetGeneralInventory)
          (:then
            (Widget|SetVisibility _generalinventory_2 "Hidden")
            (Variables|/Script/Engine.PlayerController|SetbShowMouseCursor _returnvalue false)
            (Input|SetInputModeGameOnly _returnvalue false)
            (bind _asbp_third_person_character_3 (Utilities|Casting|CastToBP_ThirdPersonCharacter (Components|GetOwner)))
            (Pawn|Components|CharacterMovement|SetMovementMode (Variables|/Script/Engine.Character|GetCharacterMovement _asbp_third_person_character_3) "MOVE_Walking" 0)
            (bind _asbp_third_person_character_4 (Utilities|Casting|CastToBP_ThirdPersonCharacter (Components|GetOwner)))
            (Variables|/Game/Blueprints/BPC_AttackSystem.BPC_AttackSystem_C|SetCanAttack? (Variables|/Game/ThirdPerson/Blueprints/BP_ThirdPersonCharacter.BP_ThirdPersonCharacter_C|GetBPC_AttackSystem _asbp_third_person_character_4) true))
          (:else))))))

(event EventBeginPlay
  (bind _asbp_third_person_character (Utilities|Casting|CastToBP_ThirdPersonCharacter (Components|GetOwner)))
  (Variables|Default|SetAs%20BP%20Third%20Person%20Character _asbp_third_person_character)
  (Variables|Default|SetFollow%20Camera (Variables|/Game/ThirdPerson/Blueprints/BP_ThirdPersonCharacter.BP_ThirdPersonCharacter_C|GetFollowCamera _asbp_third_person_character)))

(event Input|KeyboardEvents|DebugKeyH
  (params (Key :type Key%20Structure) (ActionValue :type Input%20Action%20Value%20Structure))
  ;[1 1 1] Pick Up Trace
  (:Pressed
    (for _array_element (Variables|Default|GetWeaponSlots)
      (Development|PrintString (Utilities|String|ToString(Name) (.rowname (.item _array_element)))))))

(fn AddWeapon
  (params (NewItem :type BPS%20Slots%20Structure%20%28by%20ref%29))
  (Utilities|Array|Add (Variables|Default|GetWeaponSlots) NewItem))

(fn AddConsumable
  (params (NewItem :type BPS%20Slots%20Structure))
  (Utilities|Array|Add (Variables|Default|GetConsumableSlots) NewItem))

(fn GetConsumable)