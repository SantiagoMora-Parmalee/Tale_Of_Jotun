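; BP_Door is a door actor that toggles open and closed by swinging through a quarter turn.
; Each OpenDoor call alternates through a FlipFlop between playing a timeline from the start and reversing it.
; The timeline's Door track drives a lerp that sets the door mesh's relative yaw.
; The construction script applies the DoorMesh and DoorFrameMesh variables, so the door and frame meshes are configurable.
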(event Custom|OpenDoor
  (Utilities|FlowControl|FlipFlop
    (:A
      (bind _door (Timeline|OpeningDoorTimeline PlayFromStart)
        (:Update
          (Transformation|SetRelativeRotation (Variables|Default|GetDoor) (Math|Rotator|MakeRotator 0.0 0.0 (Math|Float|Lerp -9e+01 0.0 _door)) false false))))
    (:B
      (Timeline|OpeningDoorTimeline Reverse))))

(event EventBeginPlay)

(event Collision|EventActorBeginOverlap
  (params (OtherActor :type Actor%20Object%20Reference)))

(event EventTick
  (params (DeltaSeconds :type Float%20%28single-precision%29)))

(fn ConstructionScript
  (Components|StaticMesh|SetStaticMesh (Variables|Default|GetDoor) (Variables|Default|GetDoorMesh))
  (Components|StaticMesh|SetStaticMesh (Variables|Default|GetDoorFrame) (Variables|Default|GetDoorFrameMesh)))