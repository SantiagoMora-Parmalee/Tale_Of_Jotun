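; BP_Dark_Boundary is a trigger volume that builds up the player's Dark stat while the third-person character stands inside it.
; Entering TriggerZone sets InZone and starts a Delay-driven loop calling IncreaseDark on the character's BPCPlayerStats component.
; Leaving clears the flag and, after a grace delay, starts a slower DecreaseDark loop that runs until re-entry, with no other stop condition.
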(event OnComponentBeginOverlap(TriggerZone)
  (params (OverlappedComponent :type Primitive%20Component%20Object%20Reference) (OtherActor :type Actor%20Object%20Reference) (OtherComp :type Primitive%20Component%20Object%20Reference) (OtherBodyIndex :type Integer) (bFromSweep :type Boolean) (SweepResult :type Hit%20Result%20Structure%20%28by%20ref%29))
  (bind _asbp_third_person_character (Utilities|Casting|CastToBP_ThirdPersonCharacter OtherActor))
  (Variables|Default|SetAs%20BP%20Third%20Person%20Character _asbp_third_person_character)
  (Variables|Default|SetInZone? true)
  (if (Variables|Default|GetInZone?) :!label _label
    (Default|IncreaseDark (Variables|/Game/ThirdPerson/Blueprints/BP_ThirdPersonCharacter.BP_ThirdPersonCharacter_C|GetBPC_PlayerStats (Variables|Default|GetAs%20BP%20Third%20Person%20Character)) 2.0)
    (Utilities|FlowControl|Delay 0.1)
    (goto _label)))

(event OnComponentEndOverlap(TriggerZone)
  (params (OverlappedComponent :type Primitive%20Component%20Object%20Reference) (OtherActor :type Actor%20Object%20Reference) (OtherComp :type Primitive%20Component%20Object%20Reference) (OtherBodyIndex :type Integer))
  (Utilities|Casting|CastToBP_ThirdPersonCharacter OtherActor)
  (Variables|Default|SetInZone? false)
  (if (not (Variables|Default|GetInZone?))
    (Utilities|FlowControl|Delay 3.0)
    (if (not (Variables|Default|GetInZone?)) :!label _label
      (Default|DecreaseDark (Variables|/Game/ThirdPerson/Blueprints/BP_ThirdPersonCharacter.BP_ThirdPersonCharacter_C|GetBPC_PlayerStats (Variables|Default|GetAs%20BP%20Third%20Person%20Character)) 2.0)
      (Utilities|FlowControl|Delay 0.2)
      (goto _label))))

(event EventBeginPlay
  (bind _asbp_third_person_character (Utilities|Casting|CastToBP_ThirdPersonCharacter (Components|GetOwner)))
  (Variables|Default|SetBPC%20Player%20Stats (Variables|/Game/ThirdPerson/Blueprints/BP_ThirdPersonCharacter.BP_ThirdPersonCharacter_C|GetBPC_PlayerStats _asbp_third_person_character)))

(event Collision|EventActorBeginOverlap
  (params (OtherActor :type Actor%20Object%20Reference)))

(event EventTick
  (params (DeltaSeconds :type Float%20%28single-precision%29)))

(fn ConstructionScript)