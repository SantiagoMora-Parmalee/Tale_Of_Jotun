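; Enemy character for melee combat that exposes patrol route, ideal ranges and movement speed, apparently for AI.
; Attack plays a sword montage whose notify sphere-traces forward to damage tagged players, then signals attack end.
; AnyDamage applies knockback and reduces health through BPCPlayerStats; death triggers ragdoll, hides the health bar and credits player quest and XP.
; Construction applies configurable meshes, while most health, damage and attack-token functions are stubs.
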(event Custom|Attack%202
  (Animation|Montage|PlayMontage 0 0))

(event Custom|Attack
  (bind _returnvalue (Transformation|GetActorLocation))
  (bind _notifyname (Animation|Montage|PlayMontage (Variables|Character|GetMesh) "/Game/Characters/Animations/AliZohAnims/Melee/Montage_Sword_Slash.Montage_Sword_Slash")
    (:OnCompleted
      (Default|CallOnAttackEnd :!label _label))
    (:OnInterrupted
      (goto _label))
    (:OnNotifyBegin
      (switch name _notifyname
        (:Slash
          (bind (_outhit _returnvalue_2) (Collision|SphereTraceForObjects _returnvalue (+ _returnvalue (* (Transformation|GetActorForwardVector) 2e+02)) 2e+01 (Utilities|Array|MakeArray "ObjectTypeQuery3") false 0 "ForDuration"))
          (if _returnvalue_2
            (if (Actor|ActorHasTag (.HitActor (Collision|BreakHitResult _outhit)) "DamageablePlayer")
              (Game|Damage|ApplyDamage (.HitActor (Collision|BreakHitResult _outhit)) (Variables|Default|GetDamage) 0 0))))))))

(event Custom|WieldSword
  (Transformation|AttachComponentToComponent (Components|GetOwner (Variables|Default|GetWeapon)) (Variables|Character|GetMesh) "Hand_R_Weapon" "SnapToTarget" "SnapToTarget" "SnapToTarget" true)
  (Variables|Default|SetIsWieldingSword true))

(event Game|Damage|EventAnyDamage
  (params (Damage :type Float%20%28single-precision%29) (DamageType :type Damage%20Type%20Object%20Reference) (InstigatedBy :type Controller%20Object%20Reference) (DamageCauser :type Actor%20Object%20Reference))
  (bind _asbp_third_person_character (Utilities|Casting|CastToBP_ThirdPersonCharacter (Game|GetPlayerCharacter 0)))
  (Character|LaunchCharacter (* (Math|Vector|GetForwardVector (Transformation|GetActorRotation _asbp_third_person_character)) 7e+02) false false)
  (Audio|PlaySoundatLocation "/Game/Audio/Grunts-Hits/416839__tonsil5__grunt1-death-pain.416839__tonsil5__grunt1-death-pain" (Transformation|GetActorLocation) "0, 0, 0" 1.0 (Math|Random|RandomFloatinRange 1.0 1.5) 0.0 "/Game/Audio/SA_CharacterOverall.SA_CharacterOverall" 0 0 0)
  (bind _isplayerdead_ (Default|DecreaseHealth (Variables|Default|GetBPC_PlayerStats) Damage))
  (if _isplayerdead_
    (Collision|SetCollisionObjectType (Variables|Character|GetMesh) "ECC_PhysicsBody")
    (Physics|SetSimulatePhysics (Variables|Character|GetMesh) true)
    (Audio|PlaySoundatLocation "/Game/Audio/Grunts-Hits/SC_Death.SC_Death" (Transformation|GetActorLocation) "0, 0, 0" 1.0 1.0 0.0 "/Game/Audio/SA_CharacterOverall.SA_CharacterOverall" 0 0 0)
    (Rendering|SetVisibility (Variables|Default|GetHealthBarWidget) false false)
    (Pawn|Components|CharacterMovement|SetMovementMode (Variables|Character|GetCharacterMovement) "MOVE_None" 0)
    (bind _asbp_third_person_character_2 (Utilities|Casting|CastToBP_ThirdPersonCharacter (Game|GetPlayerCharacter 0)))
    (Default|EliminateEnemy (Variables|/Game/ThirdPerson/Blueprints/BP_ThirdPersonCharacter.BP_ThirdPersonCharacter_C|GetBPC_Quests _asbp_third_person_character_2) self)
    (Default|IncreaseXP (Variables|/Game/ThirdPerson/Blueprints/BP_ThirdPersonCharacter.BP_ThirdPersonCharacter_C|GetBPC_PlayerStats _asbp_third_person_character_2) (Variables|Default|GetAdded%20XP%20for%20enemy%20death))))

(event Collision|EventActorBeginOverlap
  (params (OtherActor :type Actor%20Object%20Reference)))

(event EventTick
  (params (DeltaSeconds :type Float%20%28single-precision%29)))

(event EventBeginPlay
  (bind _aswb_dummy_healthbar (Utilities|Casting|CastToWB_DummyHealthbar (UserInterface|GetWidget (Variables|Default|GetHealthBarWidget))))
  (Variables|Default|SetWidgetHealthUi _aswb_dummy_healthbar))

(fn ConstructionScript
  (Components|StaticMesh|SetStaticMesh (Variables|Default|GetWeapon) (Variables|Default|GetWeaponMesh))
  (Components|SkeletalMesh|SetSkeletalMeshAsset (Variables|Default|GetRealEnemy) (Variables|Default|GetRealEnemyMesh)))

(fn GetIdealRange
  (return 1.5e+02 3.5e+02))

(fn GetPatrolRoute
  (return (Variables|Ai|GetPatrolRoute)))

(fn GetCurrentHealth
  (return 0.0))

(fn GetMaxHealth
  (return 0.0))

(fn GetTeamNumber
  (return 0))

(fn Heal
  (params (Amount :type Float%20%28double-precision%29))
  (return 0.0))

(fn IsAttacking
  (return false))

(fn IsDead
  (return false))

(fn ReserveAttackToken
  (params (Amount :type Integer))
  (return false))

(fn SetMovementSpeed
  (params (Speed :type E_MovementSpeed%20Enum :default "NewEnumerator0"))
  (bind _output_get (Variables|/Script/Engine.CharacterMovementComponent|SetMaxWalkSpeed (Variables|Character|GetCharacterMovement) (Utilities|Select :Index Speed :NewEnumerator0 0.0 :NewEnumerator1 1e+02 :NewEnumerator2 3e+02 :NewEnumerator3 5e+02)))
  (return _output_get))

(fn TakeDamage
  (params (DamageInfo :type S%20Damage%20Info%20Structure) (Damage%20Causer :type Actor%20Object%20Reference))
  (return false))