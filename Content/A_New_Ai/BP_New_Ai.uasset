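; AI character Blueprint that provides melee attack, sword wielding, patrol route and movement speed functions.
; Attack plays a montage and calls OnAttackEnd whether it completes or is interrupted.
; The construction script sets the weapon mesh, and WieldSword attaches to the right-hand socket and flags the sword as wielded.
; SetMovementSpeed maps idle, walk, jog and run states to max walk speed, while GetPatrolRoute exposes the assigned route.
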(event Custom|Attack
  (Animation|Montage|PlayMontage (Variables|Character|GetMesh) "/Game/Characters/Animations/SwordCombat/Attack1_Montage.Attack1_Montage"
    (:OnCompleted
      _)
    (:OnInterrupted
      _))
  (Default|CallOnAttackEnd))

(event Custom|WieldSword
  (Transformation|AttachComponentToComponent (Components|GetOwner (Variables|Default|GetWeapon)) (Variables|Character|GetMesh) "Hand_R_Weapon" "SnapToTarget" "SnapToTarget" "SnapToTarget" true)
  (Variables|Default|SetIsWieldingSword true))

(event EventBeginPlay)

(event Collision|EventActorBeginOverlap
  (params (OtherActor :type Actor%20Object%20Reference)))

(event EventTick
  (params (DeltaSeconds :type Float%20%28single-precision%29)))

(fn ConstructionScript
  (Components|StaticMesh|SetStaticMesh (Variables|Default|GetWeapon) (Variables|Default|GetWeaponMesh)))

(fn GetPatrolRoute
  (return (Variables|Ai|GetPatrolRoute)))

(fn SetMovementSpeed
  (params (Speed :type E_MovementSpeed%20Enum :default "NewEnumerator0"))
  (bind _output_get (Variables|/Script/Engine.CharacterMovementComponent|SetMaxWalkSpeed (Variables|Character|GetCharacterMovement) (Utilities|Select :Index Speed :NewEnumerator0 0.0 :NewEnumerator1 1e+02 :NewEnumerator2 3e+02 :NewEnumerator3 5e+02)))
  (return _output_get))