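; Openable chest actor that gives the player an item and XP once, with its top and base meshes set in the construction script.
; The Open Chest function uses a ChestOpened guard, fires the animation event, notifies the character's quest component, adds XP to player stats and returns Item.
; The event uses a FlipFlop to play or reverse a timeline that lerps the roll of ChestBase.
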(event Custom|OpenChest
  (Utilities|FlowControl|FlipFlop
    (:A
      (bind _chestopening (Timeline|OpeningChest Play)
        (:Update
          (Transformation|SetRelativeRotation (Variables|Default|GetChestBase) (Math|Rotator|MakeRotator (Math|Float|Lerp 0.0 -2.4e+02 _chestopening) 0.0 0.0) false false))))
    (:B
      (Timeline|OpeningChest Reverse))))

(event EventBeginPlay)

(event Collision|EventActorBeginOverlap
  (params (OtherActor :type Actor%20Object%20Reference)))

(event EventTick
  (params (DeltaSeconds :type Float%20%28single-precision%29)))

(fn ConstructionScript
  (Components|StaticMesh|SetStaticMesh (Variables|Default|GetChestTop) (Variables|Default|GetChestTopMesh))
  (Components|StaticMesh|SetStaticMesh (Variables|Default|GetChestBase) (Variables|Default|GetChestBaseMesh)))

(fn OpenChest
  (if (not (Variables|Default|GetChestOpened?))
    (Variables|Default|SetChestOpened? true)
    (CallFunction|OpenChest)
    (bind _asbp_third_person_character (Utilities|Casting|CastToBP_ThirdPersonCharacter (Game|GetPlayerCharacter 0)))
    (Default|OpenChest (Variables|/Game/ThirdPerson/Blueprints/BP_ThirdPersonCharacter.BP_ThirdPersonCharacter_C|GetBPC_Quests _asbp_third_person_character) self)
    (Default|IncreaseXP (Variables|/Game/ThirdPerson/Blueprints/BP_ThirdPersonCharacter.BP_ThirdPersonCharacter_C|GetBPC_PlayerStats _asbp_third_person_character) (Variables|Default|GetAdded%20XP))
    (return (Variables|Default|GetItem))))