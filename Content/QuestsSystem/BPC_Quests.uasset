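; Quest component that tracks the active quest's objectives and displays their progress in a quest HUD widget it creates on BeginPlay.
; EliminateEnemy removes enemies from a shared working array until it empties, while OpenChest matches the opened chest against chest objectives.
; Both update objective structs by reference, notify the widget and call ObjectiveCompleted, which counts completions, then clears the quest and plays the completion animation once all are done.
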(event Custom|Set%20Active%20Quest%20Text
  (Rendering|Components|TextRender|SetText (Variables|/Game/QuestsSystem/UI_Quest.UI_Quest_C|GetActiveQuestText (Variables|Default|GetQuest%20Hud%20Widget)) (Utilities|Text|ToText(String) (.Name (Utilities|Struct|BreakBPS_Quests (Variables|Default|GetActiveQuest)))))
  (Default|ShowQuestPanel (Variables|Default|GetQuest%20Hud%20Widget)))

(event Custom|Set%20Objectives
  (Default|FillObjectives (Variables|Default|GetQuest%20Hud%20Widget) (.objectives (Variables|Default|GetActiveQuest))))

(event Custom|EliminateEnemy
  (params (EnemyElimination :type Actor%20Object%20Reference))
  (for _array_element (.objectives (Variables|Default|GetActiveQuest))
    (if (and (not (.Completed (Utilities|Struct|BreakS_QuestObjective _array_element))) (.IsEliminateEnemyObjective (Utilities|Struct|BreakS_QuestObjective _array_element)))
      (if (!= (Utilities|Array|Length (Variables|Default|GetenemyActorsArray)) 0)
        _
        (else
          (bind _output_get (Variables|Default|SetenemyActorsArray (.ActorsToEliminate (Utilities|Struct|BreakS_QuestObjective _array_element))))))
      (Utilities|Array|RemoveItem _output_get EnemyElimination)
      (|SetBy-RefVar _array_element (Utilities|Struct|MakeS_QuestObjective (.Name (Utilities|Struct|BreakS_QuestObjective _array_element)) false (Variables|Default|GetenemyActorsArray) (.ChestToOPen (Utilities|Struct|BreakS_QuestObjective _array_element)) (.IsEliminateEnemyObjective (Utilities|Struct|BreakS_QuestObjective _array_element)) (.IsChestObjective (Utilities|Struct|BreakS_QuestObjective _array_element))))
      (Development|PrintString (Utilities|String|ToString(Integer) (Utilities|Array|Length (Variables|Default|GetenemyActorsArray))))
      (if (== (Utilities|Array|Length (Variables|Default|GetenemyActorsArray)) 0)
        (|SetBy-RefVar _array_element (Utilities|Struct|MakeS_QuestObjective (.Name (Utilities|Struct|BreakS_QuestObjective _array_element)) true "(None)" (.ChestToOPen (Utilities|Struct|BreakS_QuestObjective _array_element)) (.IsEliminateEnemyObjective (Utilities|Struct|BreakS_QuestObjective _array_element)) (.IsChestObjective (Utilities|Struct|BreakS_QuestObjective _array_element))))
        (Default|CompleteObjective (Variables|Default|GetQuest%20Hud%20Widget) _array_element)
        (CallFunction|ObjectiveCompleted)
        (Development|PrintString "Completed")))))

(event Custom|Open%20Chest
  (params (Chest :type Actor%20Object%20Reference))
  (for _array_element (.objectives (Variables|Default|GetActiveQuest))
    (if (and (.IsChestObjective (Utilities|Struct|BreakS_QuestObjective _array_element)) (== Chest (.ChestToOPen (Utilities|Struct|BreakS_QuestObjective _array_element))))
      (|SetBy-RefVar _array_element (Utilities|Struct|MakeS_QuestObjective (.Name (Utilities|Struct|BreakS_QuestObjective _array_element)) true (.ActorsToEliminate (Utilities|Struct|BreakS_QuestObjective _array_element)) 0 (.IsEliminateEnemyObjective (Utilities|Struct|BreakS_QuestObjective _array_element)) (.IsChestObjective (Utilities|Struct|BreakS_QuestObjective _array_element))))
      (Default|CompleteObjective (Variables|Default|GetQuest%20Hud%20Widget) _array_element)
      (CallFunction|ObjectiveCompleted)
      (Development|PrintString "Completed"))))

(event Custom|Objective%20Completed
  (Math|Integer|IncrementInt (Variables|Default|GetObjectivesCompleted)
    (:%20%20
      (if (>= (Variables|Default|GetObjectivesCompleted) (Utilities|Array|Length (.objectives (Variables|Default|GetActiveQuest))))
        (Development|PrintString "Quest completed")
        (Variables|Default|SetActiveQuest "")
        (Variables|Default|SetObjectivesCompleted 0)
        (Default|QuestCompletedAnimation (Variables|Default|GetQuest%20Hud%20Widget))))))

(event EventBeginPlay
  (bind _returnvalue (UserInterface|CreateWidget "/Game/QuestsSystem/UI_Quest.UI_Quest_C"))
  (bind _output_get (Variables|Default|SetQuest%20Hud%20Widget _returnvalue))
  (UserInterface|Viewport|AddtoViewport _output_get 0)
  (Default|HideQuestPanel (Variables|Default|GetQuest%20Hud%20Widget)))

(event EventTick
  (params (DeltaSeconds :type Float%20%28single-precision%29)))